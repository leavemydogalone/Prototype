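; GA_SelectAbility is a player gameplay ability that selects the unit under the mouse cursor.
; A TargetDataUnderMouse task supplies the hit result, and the hit actor is passed to SetSelectedUnit on the AuraPlayerState.
; The player state is resolved from the avatar pawn on first use and cached, and the ability ends after a half-second delay.
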(event Ability|EventActivateAbility
  (bind _datahandle (|TargetDataUnderMouse)
    (:ValidData
      (Utilities|IsValid (Variables|Default|GetAuraPlayerState)
        (:Is%20Valid
          _)
        (:Is%20Not%20Valid
          (bind _aspawn (Utilities|Casting|CastToPawn (Ability|GetAvatarActorfromActorInfo)))
          (bind _asaura_player_state (Utilities|Casting|CastToAuraPlayerState (Variables|/Script/Engine.Pawn|GetPlayerState _aspawn)))
          (bind _output_get (Variables|Default|SetAuraPlayerState _asaura_player_state))))
      (Class|AuraPlayerState|SetSelectedUnit _output_get (.HitActor (Collision|BreakHitResult (Ability|TargetData|GetHitResultfromTargetData _datahandle))))
      (Ability|Tasks|WaitDelay 0.5
        (:then
          (Ability|EndAbility))))))

(event Ability|EventOnEndAbility
  (params (bWasCancelled :type Boolean)))