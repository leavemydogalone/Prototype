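; Gameplay ability for a unit's basic melee attack, damaging live players in a box at a combat socket.
; It turns the unit toward the confirmed target location, then plays a random tagged montage.
; The montage's gameplay event triggers the box query, applying damage and blood effects and ending the ability on a hit; montage end also ends it.
; The friend check and melee impact cue are disconnected.
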(event EventActivateUnitAbility
  (bind _returnvalue (Ability|GetAvatarActorfromActorInfo))
  (Variables|Default|SetHasHitTarget false)
  (Utilities|IsValid (Utilities|ToObject(Interface) (Variables|Default|GetSelf%20Combat%20Interface))
    (:Is%20Valid
      (Class|CombatInterface|UpdateFacingTarget (stale _output_get_3) (.Location (Collision|BreakHitResult (Ability|TargetData|GetHitResultfromTargetData (.TargetData (Utilities|Struct|BreakGameplayEventData (Variables|Default|GetConfirmedEventData)))))) :!label _label)
      (bind _returnvalue_2 (Class|CombatInterface|GetAttackMontages(Message) (Ability|GetAvatarActorfromActorInfo)))
      (bind _output_get (Variables|Default|SetTaggedMontage (Class|UnitDamageGameplayAbility|GetRandomTaggedMontagefromArray _returnvalue_2)))
      (|PlayMontageandWaitProxy "None" (.Montage (Utilities|Struct|BreakTaggedMontage _output_get)) 1.0 "None" false 1.0 0.0 false
        (:then
          (Ability|Tasks|WaitGameplayEvent (.MontageTag (Utilities|Struct|BreakTaggedMontage _output_get)) 0
            (:EventReceived
              (bind _returnvalue_3 (Class|CombatInterface|GetCombatSocketLocation(Message) _returnvalue (.SocketTag (Utilities|Struct|BreakTaggedMontage _output_get))))
              (bind _output_get_2 (Variables|Default|SetCombatSocketLocation _returnvalue_3))
              (bind _outactors (Class|AuraAbilitySystemLibrary|GetLivePlayersWithinBox (Ability|GetAvatarActorfromActorInfo) (Utilities|Array|MakeArray _returnvalue) (Variables|Default|GetBoxHalfExtent) (Variables|Default|GetBoxCenterOffset) _output_get_2 (Transformation|GetActorRotation (Ability|GetAvatarActorfromActorInfo))))
              (for _array_element _outactors
                (Class|AuraAbilitySystemLibrary|ApplyDamageEffect (Class|UnitDamageGameplayAbility|MakeDamageEffectParamsfromClassDefaults _array_element "0, 0, 0" false "0, 0, 0" false "0, 0, 0" false 0.0))
                (Variables|Default|SetHasHitTarget true)
                (Class|CombatInterface|GetBloodEffect(Message) _array_element)
                (Ability|EndAbility)))))
        (:OnCompleted
          (Ability|EndAbility :!label _label_2))
        (:OnInterrupted
          (goto _label_2))
        (:OnCancelled
          (goto _label_2))))
    (:Is%20Not%20Valid
      (bind _ascombat_interface (Utilities|Casting|CastToCombatInterface (Ability|GetAvatarActorfromActorInfo))
        (:then
          (bind _output_get_3 (Variables|Default|SetSelf%20Combat%20Interface _ascombat_interface))
          (goto _label))
        (:CastFailed
          (Ability|CancelAbility))))))