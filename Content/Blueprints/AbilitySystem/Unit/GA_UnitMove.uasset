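; Gameplay ability that moves an AI-controlled unit a short step toward a targeted point.
; ActivateUnitAbility takes the hit from event target data, projects a goal up to 500 units horizontally from the avatar in that direction, and runs AIMoveTo, ending on finish or failure.
; On event activation, the authority also listens for Event.Unit.Cancel to cancel the ability and ends it after a three-second timeout.
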(event Ability|EventOnEndAbility
  (params (bWasCancelled :type Boolean)))

(event Ability|EventActivateAbilityFromEvent
  (params (EventData :type Gameplay%20Event%20Data%20Structure%20%28by%20ref%29))
  (Ability|HasAuthority
    (:True
      (Ability|Tasks|WaitGameplayEvent "(TagName=\"Event.Unit.Cancel\")" 0
        (:then
          (Utilities|FlowControl|Delay 3.0)
          (Ability|EndAbility))
        (:EventReceived
          (Ability|CancelAbility))))))

(event EventActivateUnitAbility
  (bind _destination (CallFunction|GetTargetDestinationfromActorLocation (Ability|TargetData|GetHitResultfromTargetData (.TargetData (Utilities|Struct|BreakGameplayEventData (Variables|Default|GetCurrentEventData))))))
  (AI|AIMoveTo (AI|GetAIController (Ability|GetAvatarActorfromActorInfo)) _destination 0 -1.0 "Default" "Default" true true
    (:OnRequestFailed
      _)
    (:OnMoveFinished
      _))
  (Ability|EndAbility))

(fn GetTargetDestinationfromActorLocation
  (params (HitResult :type Hit%20Result%20Structure%20%28by%20ref%29))
  (return (+ (Transformation|GetActorLocation (Ability|GetAvatarActorfromActorInfo)) (* (Math|Vector|Normalize (- (.Location (Collision|BreakHitResult HitResult)) (Transformation|GetActorLocation (Ability|GetAvatarActorfromActorInfo)))) "500.000000,500.000000,0.000000"))))