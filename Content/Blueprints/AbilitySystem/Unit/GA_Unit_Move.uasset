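; Gameplay ability that AI-moves a unit toward the targeted location, limited to a reachable point within ability range.
; An attached trigger sphere applies damage to the first overlapping UnitInterface actor, then destroys itself.
; The ability ends when the move finishes or fails, destroying any remaining sphere.
; It draws a debug sphere at the goal; the range-clamp helper and path-preview nodes are not used by the live flow.
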(event Custom|OnActorBeginOverlap_Event
  (params (OverlappedActor :type Actor%20Object%20Reference) (OtherActor :type Actor%20Object%20Reference))
  (bind _spawned_actor (Variables|Default|GetSpawned%20Actor))
  (if (Utilities|DoesObjectImplementInterface OtherActor "/Script/Aura.UnitInterface")
    (Class|AuraAbilitySystemLibrary|ApplyDamageEffect (Class|UnitDamageGameplayAbility|MakeDamageEffectParamsfromClassDefaults OtherActor "0, 0, 0" false "0, 0, 0" false "0, 0, 0" true 3e+01))
    (Utilities|IsValid _spawned_actor
      (:Is%20Valid
        (Actor|DestroyActor _spawned_actor)))))

(event Ability|EventOnEndAbility
  (params (bWasCancelled :type Boolean))
  (bind _spawned_actor (Variables|Default|GetSpawned%20Actor))
  (Utilities|IsValid _spawned_actor
    (:Is%20Valid
      (Actor|DestroyActor _spawned_actor))))

(event EventActivateUnitAbility
  (bind _returnvalue (Ability|GetAvatarActorfromActorInfo))
  (bind _confirmedeventdata (Variables|Default|GetConfirmedEventData))
  (bind _abilityrange (Variables|Default|GetAbilityRange))
  (bind _targetdata (Utilities|Struct|BreakGameplayEventData _confirmedeventdata))
  (bind _returnvalue_2 (Transformation|GetActorLocation _returnvalue))
  (bind _returnvalue_3 (Ability|TargetData|GetHitResultfromTargetData _targetdata))
  (bind _location (Collision|BreakHitResult _returnvalue_3))
  (bind _outlocation (Class|AuraAbilitySystemLibrary|GetReachablePointWithinMaxRange _returnvalue _returnvalue_2 _location _abilityrange))
  (bind _spawnedactor (|SpawnActor :Class "/Game/Blueprints/AbilitySystem/Unit/BP_TriggerSphere.BP_TriggerSphere_C" :Instigator 0)
    (:then
      (Rendering|Debug|DrawDebugSphere _outlocation 1e+02 12 "(R=1.000000,G=1.000000,B=1.000000,A=1.000000)" 5.0)
      (AI|AIMoveTo (AI|GetAIController (Ability|GetAvatarActorfromActorInfo)) _outlocation 0 -1.0 "Default" "Default" true true
        (:OnRequestFailed
          _)
        (:OnMoveFinished
          _))
      (Ability|EndAbility))
    (:Success
      (bind _output_get (Variables|Default|SetSpawned%20Actor _spawnedactor))
      (Transformation|AttachActorToActor _output_get (Ability|GetAvatarActorfromActorInfo) "None" "KeepWorld" "KeepRelative" "KeepRelative" true)
      (EventDispatchers|AssignOnActorBeginOverlap (Variables|Default|GetSpawned%20Actor) (delegate Custom|OnActorBeginOverlap_Event)))))

(fn ClampTargetDestinationtoAbilityRange
  (params (HitResult :type Hit%20Result%20Structure%20%28by%20ref%29) (InLocation :type Vector))
  ;[1 1 1] Direction
  (LocalVariables|SetNormalizedDirection (Math|Vector|Normalize (- InLocation (Transformation|GetActorLocation (Ability|GetAvatarActorfromActorInfo)))))
  (return (+ (Transformation|GetActorLocation (Ability|GetAvatarActorfromActorInfo)) (* (LocalVariables|GetNormalizedDirection) (Math|Float|Min(Float) (Variables|Default|GetAbilityRange) (Math|Vector|VectorLength (- InLocation (Transformation|GetActorLocation (Ability|GetAvatarActorfromActorInfo)))))))))