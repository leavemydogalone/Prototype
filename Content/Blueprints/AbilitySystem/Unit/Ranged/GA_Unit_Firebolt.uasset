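; GA_Unit_Firebolt is a ranged unit gameplay ability that fires a projectile at a confirmed target location.
; On activation it caches the avatar's combat interface, cancelling if there is none, turns the unit toward the target and plays a random tagged attack montage.
; The montage's gameplay event triggers the projectile spawn from the tagged socket with optional pitch override.
; The ability ends when the montage completes, is interrupted or is cancelled.
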(event EventActivateUnitAbility
  ;[1 1 1] Will want to make a re-usable function for this, in base unit ga
  (Utilities|IsValid (Utilities|ToObject(Interface) (Variables|Default|GetSelf%20Combat%20Interface))
    (:Is%20Valid
      (bind _output_get (Variables|Default|SetConfirmedTargetLocation (.Location (Collision|BreakHitResult (Ability|TargetData|GetHitResultfromTargetData (.TargetData (Utilities|Struct|BreakGameplayEventData (Variables|Default|GetConfirmedEventData)))))) :!label _label))
      (Class|CombatInterface|UpdateFacingTarget (stale _output_get_3) _output_get)
      (bind _returnvalue (Class|CombatInterface|GetAttackMontages(Message) (Ability|GetAvatarActorfromActorInfo)))
      (bind _output_get_2 (Variables|Default|SetTaggedMontage (Class|UnitDamageGameplayAbility|GetRandomTaggedMontagefromArray _returnvalue)))
      (|PlayMontageandWaitProxy "None" (.Montage (Utilities|Struct|BreakTaggedMontage _output_get_2)) 1.0 "None" false 1.0 0.0 false
        (:then
          (Ability|Tasks|WaitGameplayEvent (.MontageTag (Utilities|Struct|BreakTaggedMontage _output_get_2)) 0 true
            (:EventReceived
              (Class|UnitProjectileSpell|SpawnProjectile (Variables|Default|GetConfirmedTargetLocation) (.SocketTag (Utilities|Struct|BreakTaggedMontage _output_get_2)) (Variables|Default|GetShouldOverridePitch) (Variables|Default|GetPitchOverride)))))
        (:OnCompleted
          (Ability|EndAbility :!label _label_2))
        (:OnInterrupted
          (goto _label_2))
        (:OnCancelled
          (goto _label_2))))
    (:Is%20Not%20Valid
      (bind _ascombat_interface (Utilities|Casting|CastToCombatInterface (Ability|GetAvatarActorfromActorInfo))
        (:then
          (bind _output_get_3 (Variables|Default|SetSelf%20Combat%20Interface _ascombat_interface))
          (goto _label))
        (:CastFailed
          (Ability|CancelAbility))))))