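; GA_Select is a Gameplay Ability that selects the player's own unit under the mouse during the Planning turn phase, and cancels in any other phase.
; It uses a TargetDataUnderMouse task and selects the hit actor if it shares the avatar's owner, ending after a short delay.
; Any other hit, or none, clears the selection and ends immediately.
; Phase checks and selection changes go through message calls to the game state and avatar.
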(event Ability|EventActivateAbility
  (bind _returnvalue (Class|TurnSystemInterface|GetCurrentTurnPhase(Message) (Game|GetGameState)))
  (if (Utilities|Enum|Equal(Enum) _returnvalue "Planning")
    (bind _datahandle (|TargetDataUnderMouse)
      (:ValidData
        (Utilities|IsValid (.HitActor (Collision|BreakHitResult (Ability|TargetData|GetHitResultfromTargetData _datahandle)))
          (:Is%20Valid
            (bind _output_get (Variables|Default|SetHit%20Actor (.HitActor (Collision|BreakHitResult (Ability|TargetData|GetHitResultfromTargetData _datahandle)))))
            (if (== (Components|GetOwner _output_get) (Components|GetOwner (Ability|GetAvatarActorfromActorInfo)))
              (Class|PlayerInterface|SetSelectedUnit(Message) (Ability|GetAvatarActorfromActorInfo) (Variables|Default|GetHit%20Actor))
              (Ability|Tasks|WaitDelay 0.1
                (:OnFinish
                  (Ability|EndAbility)))
              (else
                (Class|PlayerInterface|UnselectCurrentSelectedUnit(Message) (Ability|GetAvatarActorfromActorInfo))
                (Ability|EndAbility))))
          (:Is%20Not%20Valid
            (Class|PlayerInterface|UnselectCurrentSelectedUnit(Message) (Ability|GetAvatarActorfromActorInfo))
            (Ability|EndAbility)))))
    (else
      (Ability|CancelAbility))))