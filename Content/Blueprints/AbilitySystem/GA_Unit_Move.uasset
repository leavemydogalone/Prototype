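; GA_Unit_Move is a gameplay ability that moves a unit toward a targeted location when the turn phase changes.
; Event activation caches the Aura game state and binds to its turn phase delegate, without checking which phase arrives.
; AI MoveTo then drives the avatar up to 500 units horizontally along the direction to the event's target-data hit, regardless of target distance.
; Completion or failure ends the ability, which unbinds the delegate.
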(event Custom|Turn%20Phase%20Changed
  (params (NewTurnPhase :type EAuraTurnPhase%20Enum :default "Planning"))
  ;[1 1 1] Probably want to move all of this to either the base unit ability, or the library
  (AI|AIMoveTo (AI|GetAIController (Ability|GetAvatarActorfromActorInfo)) (+ (Transformation|GetActorLocation (Ability|GetAvatarActorfromActorInfo)) (* (Math|Vector|Normalize (- (.Location (Collision|BreakHitResult (Ability|TargetData|GetHitResultfromTargetData (.TargetData (Utilities|Struct|BreakGameplayEventData (Variables|Default|GetCurrentEventData)))))) (Transformation|GetActorLocation (Ability|GetAvatarActorfromActorInfo)))) "500.000000,500.000000,0.000000")) 0 -1.0 "Default" "Default" true true
    (:OnRequestFailed
      _)
    (:OnMoveFinished
      _))
  (Ability|EndAbility))

(event Ability|EventActivateAbility)

(event Ability|EventOnEndAbility
  (params (bWasCancelled :type Boolean))
  ;[1 1 1] Probably want to move all of this to either the base unit ability, or the library
  (EventDispatchers|UnbindEventfromOnTurnPhaseChangeDelegate (Variables|Default|GetAs%20Aura%20Game%20State%20Base) (delegate Custom|Turn%20Phase%20Changed)))

(event Ability|EventActivateAbilityFromEvent
  (params (EventData :type Gameplay%20Event%20Data%20Structure%20%28by%20ref%29))
  ;[1 1 1] Probably want to move all of this to either the base unit ability, or the library
  (Utilities|IsValid (Variables|Default|GetAs%20Aura%20Game%20State%20Base)
    (:Is%20Valid
      _)
    (:Is%20Not%20Valid
      (bind _asaura_game_state_base (Utilities|Casting|CastToAuraGameStateBase (Game|GetGameState)))
      (bind _output_get (Variables|Default|SetAs%20Aura%20Game%20State%20Base _asaura_game_state_base))))
  (EventDispatchers|BindEventtoOnTurnPhaseChangeDelegate _output_get (delegate Custom|Turn%20Phase%20Changed)))