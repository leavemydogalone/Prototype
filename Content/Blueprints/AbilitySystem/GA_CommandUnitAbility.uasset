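; Gameplay ability that issues a command to the selected unit during the Planning turn phase, and cancels outside that phase or with no unit selected.
; It takes target data under the mouse and sends it to the unit as a gameplay event, with the avatar's turn-phase tag as instigator tag.
; It then stays active to block selection until a Confirm or Cancel ability activates.
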(event Ability|EventActivateAbility
  (bind _returnvalue (Ability|GetAvatarActorfromActorInfo))
  (bind _returnvalue_2 (Class|TurnSystemInterface|GetCurrentTurnPhase(Message) (Game|GetGameState)))
  (if (Utilities|Enum|Equal(Enum) _returnvalue_2 "Planning")
    (bind _datahandle (|TargetDataUnderMouse)
      (:ValidData
        (bind _returnvalue_3 (Class|PlayerInterface|GetTurnPhaseTagtoSendtoUnit(Message) (Ability|GetAvatarActorfromActorInfo)))
        (Development|PrintString (Utilities|String|ToString(Name) (GameplayTags|GetTagName _returnvalue_3)))
        (bind _returnvalue_4 (Class|PlayerInterface|GetSelectedUnit(Message) _returnvalue))
        (Utilities|IsValid _returnvalue_4
          (:Is%20Valid
            (Ability|SendGameplayEventtoActor _returnvalue_4 (Variables|Default|GetOutputTag) (Utilities|Struct|MakeGameplayEventData "(TagName=\"\")" _returnvalue 0 0 0 "()" (GameplayTags|MakeGameplayTagContainerfromTag _returnvalue_3) "(GameplayTags=)" 0.0 _datahandle))
            ;[1 1 1] Keep ability active until one of these happens, so we can block the Select ability, and only allow confirm to fire
            (|WaitforAbilityActivate :WithTag "(TagName=\"Abilities.Cancel\")"
              (:then
                (|WaitforAbilityActivate :WithTag "(TagName=\"Abilities.Confirm\")"
                  (:OnActivate
                    _)))
              (:OnActivate
                _))
            (Ability|EndAbility))
          (:Is%20Not%20Valid
            (Ability|CancelAbility)))))
    (else
      (Ability|CancelAbility))))

(event Ability|EventOnEndAbility
  (params (bWasCancelled :type Boolean)))