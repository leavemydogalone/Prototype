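; GA_SelectAbility is a Gameplay Ability that selects the unit under the mouse.
; On activation it sends an Event.Unit.Cancel gameplay event to the currently selected unit, then gets the hit actor from a TargetDataUnderMouse task.
; If that actor shares the avatar's owner, it becomes the selected unit and the ability ends after a short delay; otherwise the ability ends immediately.
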(event Ability|EventActivateAbility
  ;[1 1 1] Need to figure out how to just apply GE_Cancel
  (bind _returnvalue (Class|PlayerInterface|GetSelectedUnit(Message) (Ability|GetAvatarActorfromActorInfo)))
  (Ability|SendGameplayEventtoActor _returnvalue "(TagName=\"Event.Unit.Cancel\")")
  (bind _datahandle (|TargetDataUnderMouse)
    (:ValidData
      (if (== (Components|GetOwner (Ability|GetAvatarActorfromActorInfo)) (Components|GetOwner (.HitActor (Collision|BreakHitResult (Ability|TargetData|GetHitResultfromTargetData _datahandle)))))
        (Class|PlayerInterface|SetSelectedUnit(Message) (Ability|GetAvatarActorfromActorInfo) (.HitActor (Collision|BreakHitResult (Ability|TargetData|GetHitResultfromTargetData _datahandle))))
        (Ability|Tasks|WaitDelay 0.5
          (:OnFinish
            (Ability|EndAbility)))
        (else
          (Ability|EndAbility))))))

(event Ability|EventOnEndAbility
  (params (bWasCancelled :type Boolean)))