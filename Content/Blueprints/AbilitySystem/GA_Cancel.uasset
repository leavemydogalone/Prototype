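; GA_Cancel is a gameplay ability that handles the cancel input for the avatar actor.
; If a selected unit message exists, it sends an Event.Unit.Cancel gameplay event to that actor and prints a debug string.
; Otherwise the server removes the avatar's last stored ability message, while clients cancel the ability.
; Outside that client cancel, the ability waits for input release before ending.
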(event Ability|EventActivateAbility
  (bind _returnvalue (Class|PlayerInterface|GetSelectedUnit(Message) (Ability|GetAvatarActorfromActorInfo)))
  (Utilities|IsValid _returnvalue
    (:Is%20Valid
      (Ability|SendGameplayEventtoActor _returnvalue "(TagName=\"Event.Unit.Cancel\")")
      (Development|PrintString "cancel")
      (Ability|Tasks|WaitInputRelease false :!label _label
        (:OnRelease
          (Ability|EndAbility))))
    (:Is%20Not%20Valid
      (if (Networking|IsServer)
        (Class|PlayerInterface|RemoveLastStoredAbility(Message) (Ability|GetAvatarActorfromActorInfo))
        (goto _label)
        (else
          (Ability|CancelAbility))))))

(event Ability|EventOnEndAbility
  (params (bWasCancelled :type Boolean)))